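; BP_Player is the player pawn or character for DinerDash, with sideways movement and an early customer-interaction check.
; The MoveRight axis adds movement input along the actor's right vector.
; Actor overlaps call CustomerInteract, which casts player pawn 0, rather than the overlapped actor, to BP_Customer.
; If that cast succeeds, it only prints whether the overlapped actor is that pawn.
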(event EventBeginPlay)

(event Collision|EventActorBeginOverlap
  (params (OtherActor :type Actor%20Object%20Reference))
  (CallFunction|CustomerInteract OtherActor))

(event EventTick
  (params (DeltaSeconds :type Float%20%28single-precision%29)))

(event Input|AxisEvents|InputAxisMoveRight
  (params (AxisValue :type Float%20%28single-precision%29))
  (Pawn|Input|AddMovementInput (Transformation|GetActorRightVector) AxisValue false))

(fn ConstructionScript
  (|CallParentFunction))

(fn CustomerInteract
  (params (otherActor :type Actor%20Object%20Reference))
  (bind _asbp_customer (Utilities|Casting|CastToBP_Customer (Game|Player|GetPlayerPawn 0)))
  (if (== otherActor _asbp_customer)
    (Development|PrintString "True")
    (else
      (Development|PrintString "False"))))